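; BP_LightBall is a temporary light ball from the player's abilities that grows in, lasts a set lifetime, then shrinks away and destroys itself.
; Tick lerps the sphere's scale up from zero on spawn and back down at the end, driven by flags and a shared timer.
; A timer calls LifetimeEnd, which starts the shrink, decrements the player's light ball count and fades out the attached, pitch-randomized looping sound.
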(event EventBeginPlay
  (Transformation|SetWorldScale3D (Variables|Default|GetSphere) "0, 0, 0")
  (Utilities|Time|SetTimerbyFunctionName 0 "LifetimeEnd" (Variables|Default|GetTotalLifetime))
  (bind _returnvalue (Audio|SpawnSoundAttached "/Game/Audio/LightBallMax.LightBallMax" (Variables|Default|GetSphere) "None" (Transformation|GetActorLocation) "0, 0, 0" "KeepRelativeOffset" false 1.0 (Math|Random|RandomFloatinRange 0.95 1.05) 0.0 "/Game/Audio/SA_Default.SA_Default" 0))
  (bind _output_get (Variables|Default|SetLightSound _returnvalue))
  (Audio|Components|Audio|FadeIn _output_get 0.5 1.0 0.0 "Linear" :!class /Script/Engine.AudioComponent))

(event EventTick
  (params (DeltaSeconds :type Float%20%28single-precision%29))
  (Utilities|FlowControl|Sequence
    (:then_0
      ;[1 1 1] Scale Up
      (if (Variables|Default|GetScaleUp)
        (bind _output_get (Variables|Default|Settimer (+ (Variables|Default|Gettimer) DeltaSeconds)))
        (Transformation|SetWorldScale3D (Variables|Default|GetSphere) (Math|Vector|Lerp(Vector) "0, 0, 0" (Variables|Default|GetNormalScale) (/ _output_get (Variables|Default|GetScaleTime))))
        (if (>= (Variables|Default|Gettimer) (Variables|Default|GetScaleTime))
          (Variables|Default|SetScaleUp false)
          (Variables|Default|Settimer 0.0))))
    (:then_1
      ;[1 1 1] Scale Down
      (if (Variables|Default|GetScaleDown)
        (bind _output_get_2 (Variables|Default|Settimer (+ (Variables|Default|Gettimer) DeltaSeconds)))
        (Transformation|SetWorldScale3D (Variables|Default|GetSphere) (Math|Vector|Lerp(Vector) (Variables|Default|GetNormalScale) "0, 0, 0" (/ _output_get_2 (Variables|Default|GetScaleTime))))
        (if (>= (Variables|Default|Gettimer) (Variables|Default|GetScaleTime))
          (Actor|DestroyActor))))))

(fn ConstructionScript)

(fn LifetimeEnd
  (Variables|Default|SetScaleDown true)
  (Default|ReduceCurrentLightBallCount (Variables|Default|GetPlayer))
  (Audio|Components|Audio|FadeOut (Variables|Default|GetLightSound) 0.5 0.0 "Linear" :!class /Script/Engine.AudioComponent))
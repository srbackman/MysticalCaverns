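; Fireball ability actor that grows in with a looping-style scale lerp on Tick and carries an attached fire sound.
; When its lifetime timer expires, it shrinks over the same scale time, then explodes with Niagara and sound and destroys itself.
; On hit it explodes immediately, first sending SetOnFireMessage to the other actor if the hit component's first tag is "Explosive".
; Both endings decrement the Player's active fireball count.
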(event OnComponentHit(Sphere)
  (params (HitComponent :type Primitive%20Component%20Object%20Reference) (OtherActor :type Actor%20Object%20Reference) (OtherComp :type Primitive%20Component%20Object%20Reference) (NormalImpulse :type Vector :default "0, 0, 0") (Hit :type Hit%20Result%20Structure%20%28by%20ref%29))
  (bind _componenttags (Variables|/Script/Engine.ActorComponent|GetComponentTags OtherComp))
  ;[1 1 1] Comment
  (if (> (Utilities|Array|Length _componenttags) 0)
    (if (== (Utilities|Array|Get(acopy) _componenttags) "Explosive")
      (Class|BPIFireInteraction|SetonFire(Message) OtherActor self)))
  (Default|ReduceCurrentFireBallCount (Variables|Default|GetPlayer))
  (Niagara|SpawnSystematLocation "/Game/Blueprints/Player/Abilities/NS_Explosion.NS_Explosion" (Transformation|GetActorLocation) (Transformation|GetActorRotation) (Transformation|GetActorScale3D))
  (Audio|PlaySoundatLocation "/Game/Audio/FireExplosionMax.FireExplosionMax" (Transformation|GetActorLocation) "0, 0, 0" 1.0 (Math|Random|RandomFloatinRange 0.85 1.05) 0.0 "/Game/Audio/SA_Default.SA_Default" 0 0 0)
  (Actor|DestroyActor))

(event EventBeginPlay
  (Transformation|SetWorldScale3D (Variables|Default|GetSphere) "0, 0, 0")
  (Utilities|Time|SetTimerbyFunctionName 0 "LifetimeEnd" (Variables|Default|GetTotalLifetime))
  (Audio|SpawnSoundAttached "/Game/Audio/FireMax.FireMax" (Variables|Default|GetSphere) "None" "0, 0, 0" "0, 0, 0" "KeepRelativeOffset" true 0.7 (Math|Random|RandomFloatinRange 0.85 1.05) 0.0 "/Game/Audio/SA_Default.SA_Default" 0))

(event EventTick
  (params (DeltaSeconds :type Float%20%28single-precision%29))
  (Utilities|FlowControl|Sequence
    (:then_0
      ;[1 1 1] Scale Up
      (if (Variables|Default|GetScaleUp)
        (bind _output_get (Variables|Default|Settimer (+ (Variables|Default|Gettimer) DeltaSeconds)))
        (Transformation|SetWorldScale3D (Variables|Default|GetSphere) (Math|Vector|Lerp(Vector) "0, 0, 0" (Variables|Default|GetNormalScale) (/ _output_get (Variables|Default|GetScaleTime))))
        (if (>= (Variables|Default|Gettimer) (Variables|Default|GetScaleTime))
          (Variables|Default|SetScaleUp false)
          (Variables|Default|Settimer 0.0))))
    (:then_1
      ;[1 1 1] Scale Down
      (if (Variables|Default|GetScaleDown)
        (bind _output_get_2 (Variables|Default|Settimer (+ (Variables|Default|Gettimer) DeltaSeconds)))
        (Transformation|SetWorldScale3D (Variables|Default|GetSphere) (Math|Vector|Lerp(Vector) (Variables|Default|GetNormalScale) "0, 0, 0" (/ _output_get_2 (Variables|Default|GetScaleTime))))
        (if (>= (Variables|Default|Gettimer) (Variables|Default|GetScaleTime))
          (Niagara|SpawnSystematLocation "/Game/Blueprints/Player/Abilities/NS_Explosion.NS_Explosion" (Transformation|GetActorLocation) (Transformation|GetActorRotation) (Transformation|GetActorScale3D))
          (Audio|PlaySoundatLocation "/Game/Audio/FireExplosionMax.FireExplosionMax" (Transformation|GetActorLocation) "0, 0, 0" 1.0 (Math|Random|RandomFloatinRange 0.85 1.05) 0.0 "/Game/Audio/SA_Default.SA_Default" 0 0 0)
          (Actor|DestroyActor))))))

(fn ConstructionScript)

(fn LifetimeEnd
  (Variables|Default|SetScaleDown true)
  (Default|ReduceCurrentFireBallCount (Variables|Default|GetPlayer)))
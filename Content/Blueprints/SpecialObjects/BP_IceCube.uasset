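; BP_IceCube is a temporary physics ice cube that floats when told it is inside a buoyant area.
; Tick scales it up from zero on spawn; after a maximum lifetime it decrements the player's ice cube count, shrinks and destroys itself.
; UpdatePlayer toggles gravity and buoyancy, which applies a constant upward force and smooths rotation toward upright with a weighted moving average.
; Spawning also plays an attached, randomly pitched sound.
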(event EventBeginPlay
  (Transformation|SetWorldScale3D (Variables|Default|GetCube) "0, 0, 0")
  (Utilities|Time|SetTimerbyFunctionName 0 "StartScaleDown" (Variables|Default|GetMaxLifetime))
  (Audio|SpawnSoundAttached "/Game/Audio/IceCubeMax.IceCubeMax" (Variables|Default|GetCube) "None" (Transformation|GetActorLocation) "0, 0, 0" "KeepRelativeOffset" false 1.0 (Math|Random|RandomFloatinRange 0.85 1.05) 0.0 0 0))

(event EventTick
  (params (DeltaSeconds :type Float%20%28single-precision%29))
  (bind _cube (Variables|Default|GetCube))
  (Utilities|FlowControl|Sequence
    (:then_0
      ;[1 1 1] Scale Up
      (if (Variables|Default|GetScaleUp)
        (bind _output_get (Variables|Default|Settimer (+ (Variables|Default|Gettimer) DeltaSeconds)))
        (Transformation|SetWorldScale3D (Variables|Default|GetCube) (Math|Vector|Lerp(Vector) "0, 0, 0" (Variables|Default|GetNormalScale) (/ _output_get (Variables|Default|GetScaleTime))))
        (if (>= (Variables|Default|Gettimer) (Variables|Default|GetScaleTime))
          (Variables|Default|SetScaleUp false)
          (Variables|Default|Settimer 0.0))))
    (:then_1
      ;[1 1 1] Buoyancy
      (if (Variables|Default|GetInsideBuoyant)
        (Physics|AddForce _cube (* "0.000000,0.000000,1.000000" (Variables|Default|GetBouyancySpeed)) "None" false)
        (Transformation|SetWorldRotation _cube (Class|KismetMathLibrary|WeightedMovingAverageFRotator (Math|Rotator|MakeRotationfromAxes (Math|Vector|GetForwardVector "0.000000,0.000000,1.000000") (Class|KismetMathLibrary|VectorRight) (Math|Vector|GetUpVector "0.000000,1.000000,0.000000")) (Transformation|GetWorldRotation _cube) 0.25) false false)))
    (:then_2
      ;[1 1 1] Scale Down
      (if (Variables|Default|GetScaleDown)
        (bind _output_get_2 (Variables|Default|Settimer (+ (Variables|Default|Gettimer) DeltaSeconds)))
        (Transformation|SetWorldScale3D (Variables|Default|GetCube) (Math|Vector|Lerp(Vector) (Variables|Default|GetNormalScale) "0, 0, 0" (/ _output_get_2 (Variables|Default|GetScaleTime))))
        (if (>= (Variables|Default|Gettimer) (Variables|Default|GetScaleTime))
          (Actor|DestroyActor))))))

(event EventUpdatePlayer
  (params (Inside :type Boolean))
  ;[1 1 1] Update Buoyancy
  (bind _output_get (Variables|Default|SetInsideBuoyant Inside))
  (Physics|SetEnableGravity (Variables|Default|GetCube) (not _output_get)))

(fn ConstructionScript)

(fn StartScaleDown
  (Variables|Default|SetScaleDown true)
  (Default|ReduceCurrentIceCubeCount (Variables|Default|GetPlayer)))
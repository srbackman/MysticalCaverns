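; BP_RockPlatform is a temporary rock platform that grows in, stays for a set lifetime, then shrinks and destroys itself.
; BeginPlay starts the lifetime timer and plays an attached ground sound at random pitch.
; Tick lerps the mesh's world scale between zero and normal for both phases.
; When the timer fires, StartScaleDown begins the shrink and immediately tells the Player to reduce its current ground platform count.
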(event EventBeginPlay
  (Utilities|Time|SetTimerbyFunctionName 0 "StartScaleDown" (Variables|Default|GetLifetime))
  (Audio|SpawnSoundAttached "/Game/Audio/GroundMax.GroundMax" (Variables|Default|GetRockPlatform) "None" (Transformation|GetActorLocation) "0, 0, 0" "KeepRelativeOffset" false 1.0 (Math|Random|RandomFloatinRange 0.85 1.05) 0.0 0 0))

(event EventTick
  (params (DeltaSeconds :type Float%20%28single-precision%29))
  (Utilities|FlowControl|Sequence
    (:then_0
      ;[1 1 1] Scale Up
      (if (Variables|Default|GetScaleUp)
        (bind _output_get (Variables|Default|Settimer (+ (Variables|Default|Gettimer) DeltaSeconds)))
        (Transformation|SetWorldScale3D (Variables|Default|GetRockPlatform) (Math|Vector|Lerp(Vector) "0, 0, 0" (Variables|Default|GetNormalScale) (/ _output_get (Variables|Default|GetScaleTime))))
        (if (>= (Variables|Default|Gettimer) (Variables|Default|GetScaleTime))
          (Variables|Default|SetScaleUp false)
          (Variables|Default|Settimer 0.0))))
    (:then_1
      ;[1 1 1] Scale Down
      (if (Variables|Default|GetScaleDown)
        (bind _output_get_2 (Variables|Default|Settimer (+ (Variables|Default|Gettimer) DeltaSeconds)))
        (Transformation|SetWorldScale3D (Variables|Default|GetRockPlatform) (Math|Vector|Lerp(Vector) (Variables|Default|GetNormalScale) "0, 0, 0" (/ _output_get_2 (Variables|Default|GetScaleTime))))
        (if (>= (Variables|Default|Gettimer) (Variables|Default|GetScaleTime))
          (Actor|DestroyActor))))))

(fn ConstructionScript)

(fn StartScaleDown
  (Variables|Default|SetScaleDown true)
  (Default|ReduceCurrentGroundPlatforms (Variables|Default|GetPlayer)))